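; MyPawn is a player pawn that forwards numeric keyboard input to an in-world Screen actor.
; On BeginPlay it caches the first Screen actor found in the level.
; Any key press is converted from its display name; numeric keys call NumberPressed on that Screen with the integer value.
; Non-numeric keys play an error sound at a fixed world location.
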(event EventBeginPlay
  ;[1 1 1] Gets the Screen Widget In play
  (bind _outactors (Actor|GetAllActorsOfClass "/Game/UI/UI_STUFF/Screen.Screen_C"))
  (Variables|Default|SetScreenActor (Utilities|Array|Get(acopy) _outactors)))

(event Input|KeyboardEvents|AnyKey
  (params (Key :type Key%20Structure :default "None"))
  (bind _returnvalue (Class|KismetInputLibrary|KeyGetDisplayName Key true))
  ;[1 1 1] Allows the Screen to Take Key inputs
  (:Pressed
    (if (Class|KismetStringLibrary|IsNumeric (Utilities|String|ToString(Text) _returnvalue))
      (Default|NumberPressed (Variables|Default|GetScreenActor) (Math|Conversions|ToInteger(Byte) (Utilities|String|ToString(Text) _returnvalue)))
      (else
        ;;[1 1 1] MissInput Error Sound
        (Audio|PlaySoundatLocation "/Game/UI/Sounds/Pickup_Coin.Pickup_Coin" "313.390000,-750.400000,172.830000" "0, 0, 0" 1.0 1.0 0.0 0 0 0 0)))))

(fn ConstructionScript)